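; Slide rheostat actor for the physics lab's electrical circuits, with a draggable slider that sets its resistance.
; Clicking the Cube starts a drag on Tick that follows the cursor trace along clamped local Y, interpolating Resistance from MaxResistance to zero and calling UpdateElecState.
; Electrify stores power (V²/R) in DataValue.
; MaxResistance is an editable syncable property, and the Cube is excluded from the parent's drag handling.
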(event `self.ReceiveTick`
  (params (DeltaSeconds :type "Float (single-precision)"))
  (bind _returnvalue (`GameplayStatics.GetPlayerController` 0))
  (bind _cube (`self.Cube`))
  (bind (_relativelocation_x _relativelocation_y _relativelocation_z) (`KismetMathLibrary.BreakVector` (`SceneComponent.RelativeLocation` _cube)))
  (bind _relativelocation (`SceneComponent.RelativeLocation` _cube))
  (bind (_returnvalue_x _returnvalue_y) (`KismetMathLibrary.BreakVector` (- (`.Location` (`GameplayStatics.BreakHitResult` (`PlayerController.GetHitResultUnderCursorByChannel` _returnvalue "TraceTypeQuery1" true))) (`self.K2_GetActorLocation`))))
  (bind _returnvalue_2 (`KismetMathLibrary.FClamp` _returnvalue_y -6.0 6.0))
  (`parent.ReceiveTick` DeltaSeconds)
  (if (`self.Draging`)
    (if (`PlayerController.IsInputKeyDown` _returnvalue "LeftMouseButton")
      (`SceneComponent.K2_SetRelativeLocation` _cube (`KismetMathLibrary.MakeVector` _relativelocation_x _returnvalue_2 _relativelocation_z) false false)
      (if (not (== _relativelocation (`self.LastLocation`)))
        (set `self.LastLocation` _relativelocation)
        (set `self.Resistance` (`KismetMathLibrary.Lerp` (`self.MaxResistance`) 0.0 (/ (+ _returnvalue_2 6.0) 12.0)))
        (`self.UpdateElecState`))
      (else
        (set `self.Draging` false)))))

(event `self.Cube.OnClicked`
  (params (TouchedComponent :type "PrimitiveComponent Object Reference") (ButtonPressed :type "Key Structure"))
  (set `self.Draging` true))

(event `self.Electrify`
  (params (Voltage :type "Float (single-precision)"))
  (set `self.DataValue` (* Voltage (/ Voltage (`self.Resistance`)))))

(event `self.OnPropertyValueChanged`
  (params (PropertyName :type String) (ValueStr :type String))
  (bind (_relativelocation_x _relativelocation_y) (`KismetMathLibrary.BreakVector` (`SceneComponent.RelativeLocation` (`self.Cube`))))
  (switch `string` PropertyName
    (:`MaxResistance`
      (set `self.MaxResistance` (`KismetStringLibrary.Conv_StringToDouble` ValueStr))
      (set `self.Resistance` (`KismetMathLibrary.Lerp` (`self.MaxResistance`) 0.0 (/ (+ _relativelocation_y 6.0) 12.0)))
      (`self.UpdateElecState`))))

(fn `CollectSyncableProperty`
  (returns (ReturnValue :type "Map of String to QtPropertyInfo Structure"))
  (return (`|MakeMap` "MaxResistance" (make `QtPropertyInfo` "Max Resistance" "QPT_Float" (`KismetStringLibrary.Conv_DoubleToString` (`self.MaxResistance`))))))

(fn `DragExcludeComponent`
  (returns (ReturnValue :type "Array of SceneComponent Object Reference"))
  (bind _returnvalue (`parent.DragExcludeComponent`))
  (`KismetArrayLibrary.Array_Append` _returnvalue (`|MakeArray` (`self.Cube`) :!type "SceneComponent Object Reference"))
  (return _returnvalue))

(fn `UserConstructionScript`)