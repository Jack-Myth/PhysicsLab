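; Air switch (circuit breaker) for the physics lab's electrical circuits, which trips on overcurrent.
; Clicking the lever or cube plays a timeline that rotates the lever, then sets low resistance and updates the electrical state.
; Electrify derives current from voltage and resistance; exceeding MaxCurrent triggers a short-delay Break that makes resistance near-infinite and rewinds the timeline.
; MaxCurrent is exposed as a syncable, editable property, and both clickable parts are excluded from dragging.
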(event `self.Cylinder.OnClicked`
  (params (TouchedComponent :type "PrimitiveComponent Object Reference") (ButtonPressed :type "Key Structure"))
  (bind (_direction _newtrack_0) (`Timeline|Timeline_0` :!label _label)
    (:`Update`
      (`SceneComponent.K2_SetRelativeRotation` (`self.Cylinder`) (`KismetMathLibrary.MakeRotator` 90.0 (`KismetMathLibrary.Lerp` 45.0 -45.0 _newtrack_0)) false false))
    (:`Finished`
      (set `self.Resistance` 0.1)
      (`self.UpdateElecState`))))

(event `self.Cube1.OnClicked`
  (params (TouchedComponent :type "PrimitiveComponent Object Reference") (ButtonPressed :type "Key Structure"))
  (goto _label))

(event `self.OnPropertyValueChanged`
  (params (PropertyName :type String) (ValueStr :type String))
  (switch `string` PropertyName
    (:`MaxCurrent`
      (set `self.MaxCurrent` (`KismetStringLibrary.Conv_StringToDouble` ValueStr)))))

(event `self.Electrify`
  (params (Voltage :type "Float (single-precision)"))
  (bind _returnvalue (/ Voltage (`self.Resistance`)))
  (set `self.DataValue` _returnvalue)
  (if (> _returnvalue (`self.MaxCurrent`))
    (`KismetSystemLibrary.K2_SetTimerDelegate` (delegate `Break`) 0.02)))

(event `Break`
  (set `self.Resistance` 99999997952.0)
  (`TimelineComponent.SetPlaybackPosition` (`self.Timeline_0`) 0.0 false true)
  (`self.UpdateElecState`))

(fn `CollectSyncableProperty`
  (returns (ReturnValue :type "Map of String to QtPropertyInfo Structure"))
  (return (`|MakeMap` "MaxCurrent" (make `QtPropertyInfo` "MaxCurrent" "QPT_Float" (`KismetStringLibrary.Conv_DoubleToString` (`self.MaxCurrent`))))))

(fn `DragExcludeComponent`
  (returns (ReturnValue :type "Array of SceneComponent Object Reference"))
  (bind _returnvalue (`parent.DragExcludeComponent`))
  (`KismetArrayLibrary.Array_Append` _returnvalue (`|MakeArray` (`self.Cylinder`) (`self.Cube1`) :!type "SceneComponent Object Reference"))
  (return _returnvalue))

(fn `UserConstructionScript`)